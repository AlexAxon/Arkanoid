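; BP_Block is a grid of breakable blocks that react to hits from BP_Ball.
; The construction script builds the grid from static mesh components, using X, Y and Distance for count and spacing.
; The component's material tracks damage: a first hit switches it to BasicAsset01, and a hit on that material destroys it.
; Destruction has a 50% chance to spawn a BP_Bonus, offset along X from the block.
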(event `self.ReceiveHit`
  (params (MyComp :type "PrimitiveComponent Object Reference") (Other :type "Actor Object Reference") (OtherComp :type "PrimitiveComponent Object Reference") (bSelfMoved :type Boolean) (HitLocation :type "Vector Structure") (HitNormal :type "Vector Structure") (NormalImpulse :type "Vector Structure") (Hit :type "HitResult Structure (by ref)"))
  (bind (_returnvalue_x _returnvalue_y _returnvalue_z) (`KismetMathLibrary.BreakVector` (`SceneComponent.K2_GetComponentLocation` (`self.My Comp`))))
  (set `self.My Comp` MyComp)
  (cast `/Game/Blueprints/BP_Ball` Other)
  (if (== (`PrimitiveComponent.GetMaterial` (`self.My Comp`) 0) "/Engine/MapTemplates/Materials/BasicAsset01.BasicAsset01")
    (if (== (`KismetMathLibrary.RandomIntegerInRange` 0 1) 0)
      (`|SpawnActorFromClass` "/Game/Blueprints/BP_Bonus.BP_Bonus_C" (`KismetMathLibrary.MakeTransform` (`KismetMathLibrary.MakeVector` (- _returnvalue_x 100.0) _returnvalue_y _returnvalue_z)) "AlwaysSpawn" "OverrideRootScale" null null)
      (`ActorComponent.K2_DestroyComponent` (`self.My Comp`))
      (else
        (`ActorComponent.K2_DestroyComponent` (`self.My Comp`))))
    (else
      (`PrimitiveComponent.SetMaterial` (`self.My Comp`) 0 "/Engine/MapTemplates/Materials/BasicAsset01.BasicAsset01"))))

(fn `UserConstructionScript`
  (bind _distance (`self.Distance`))
  (for _index (range (+ (`self.X`) 1))
    (for _index_2 (range (+ (`self.Y`) 1))
      (`AddComponent|NODE_AddStaticMeshComponent-0` :`RelativeTransform` (`KismetMathLibrary.MakeTransform` (`KismetMathLibrary.MakeVector` (`KismetMathLibrary.Conv_IntToDouble` (* _index _distance)) (`KismetMathLibrary.Conv_IntToDouble` (* _index_2 _distance))))))))