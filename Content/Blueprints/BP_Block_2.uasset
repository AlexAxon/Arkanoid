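; BP_Block_2 is a spawner actor that lays out a grid of BP_BlockMaterial actors when play begins.
; Nested loops over X and Y offset each block from the actor's location by multiples of Distance.
; Every block gets the same hardcoded world height and non-uniform scale, and always spawns regardless of collision.
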(event `self.ReceiveBeginPlay`
  (bind (_returnvalue_x _returnvalue_y) (`KismetMathLibrary.BreakVector` (`self.K2_GetActorLocation`)))
  (bind _distance (`self.Distance`))
  (for _index (range (+ (`self.X`) 1))
    (for _index_2 (range (+ (`self.Y`) 1))
      (`|SpawnActorFromClass` "/Game/Blueprints/BP_BlockMaterial.BP_BlockMaterial_C" (`KismetMathLibrary.MakeTransform` (`KismetMathLibrary.MakeVector` (+ _returnvalue_x (`KismetMathLibrary.Conv_IntToDouble` (* _index _distance))) (+ _returnvalue_y (`KismetMathLibrary.Conv_IntToDouble` (* _index_2 _distance))) 270.0) (struct) (1.5 4.0 1.75)) "AlwaysSpawn" "OverrideRootScale" null null))))

(fn `UserConstructionScript`)